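; BP_LaserDoor is a door that opens when every laser target sharing its DoorID is on.
; On BeginPlay it gathers all BP_LaserTarget actors with a matching ID and counts them.
; Each Tick it recounts the active targets, hiding the door and disabling its collision when all are on, and restoring both otherwise.
; With no matching targets the counts are equal, so the door stays open.
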(event `self.ReceiveBeginPlay`
  (bind _outactors (`GameplayStatics.GetAllActorsOfClass` "/Game/Blueprints/Laser/BP_LaserTarget.BP_LaserTarget_C"))
  (for _array_element _outactors
    (if (== (`/Game/Blueprints/Laser/BP_LaserTarget.doorID` _array_element) (`self.doorID`))
      (`/Engine/EditorBlueprintResources/StandardMacros.IncrementFloat` (`self.TotalTargetsWithSameID`)
        (:`  `
          (`KismetArrayLibrary.Array_Add` (`self.targetsWithSameId`) _array_element))))))

(event `self.ReceiveTick`
  (params (DeltaSeconds :type "Float (single-precision)"))
  (bind _door (`self.Door`))
  (bind _door_2 (`self.Door`))
  (set `self.CurrentActiveTargetsWithSameID` 0.0)
  (for _array_element (`self.targetsWithSameId`)
    (if (`/Game/Blueprints/Laser/BP_LaserTarget.IsOn` _array_element)
      (`/Engine/EditorBlueprintResources/StandardMacros.IncrementFloat` (`self.CurrentActiveTargetsWithSameID`))))
  (if (== (`self.TotalTargetsWithSameID`) (`self.CurrentActiveTargetsWithSameID`))
    (set `self.IsOpen` true)
    (`SceneComponent.SetVisibility` _door_2 false false)
    (`PrimitiveComponent.SetCollisionEnabled` _door_2 "NoCollision")
    (else
      (set `self.IsOpen` false)
      (`SceneComponent.SetVisibility` _door true false)
      (`PrimitiveComponent.SetCollisionEnabled` _door "QueryAndPhysics"))))

(fn `UserConstructionScript`)