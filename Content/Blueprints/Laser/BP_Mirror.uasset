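; BP_Mirror is a laser puzzle mirror that reflects incoming beams.
; LaserBounce spawns a same-colored BP_laser along the normal-mirrored direction, registering it with the mirror and the source's SpawnReferance.
; When a hit ends, it destroys attached lasers whose IDs contain the incoming beam's ID.
; A box overlap flags the player's presence, and LetGo passes the transform through a grid-snap helper, whose rounding nodes are unconnected.
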(event `self.Box_0.OnComponentBeginOverlap`
  (params (OverlappedComponent :type "PrimitiveComponent Object Reference") (OtherActor :type "Actor Object Reference") (OtherComp :type "PrimitiveComponent Object Reference") (OtherBodyIndex :type Integer) (bFromSweep :type Boolean) (SweepResult :type "HitResult Structure (by ref)"))
  (if (== (`GameplayStatics.GetObjectClass` OtherActor) "/Game/ThirdPerson/Blueprints/BP_ThirdPersonCharacter.BP_ThirdPersonCharacter_C")
    (set `self.IsPlayerInArea_0` true)))

(event `self.Box_0.OnComponentEndOverlap`
  (params (OverlappedComponent :type "PrimitiveComponent Object Reference") (OtherActor :type "Actor Object Reference") (OtherComp :type "PrimitiveComponent Object Reference") (OtherBodyIndex :type Integer))
  (if (== (`GameplayStatics.GetObjectClass` OtherActor) "/Game/ThirdPerson/Blueprints/BP_ThirdPersonCharacter.BP_ThirdPersonCharacter_C")
    (set `self.IsPlayerInArea_0` false)))

(event `LetGo`
  (params (GridSnapSize :type "Float (double-precision)") (rotationSnapSize :type "Float (double-precision)"))
  (bind (_outposition _outrotation) (`self.Position and rotation to grid` (`SceneComponent.K2_GetComponentLocation` (`self.DefaultSceneRoot`)) GridSnapSize (`self.K2_GetActorRotation` self) rotationSnapSize))
  (`SceneComponent.K2_SetWorldLocationAndRotation` (`self.DefaultSceneRoot`) _outposition _outrotation false false))

(fn `CalculateRotation`
  (params (ImpactPoint :type "Vector Structure") (ImpactNormal :type "Vector Structure") (TraceStart :type "Vector Structure"))
  (returns (ReturnValue :type "Rotator Structure"))
  (return (`KismetMathLibrary.MakeRotFromZ` (`KismetMathLibrary.MirrorVectorByNormal` (- ImpactPoint TraceStart) ImpactNormal))))

(fn `ClearAtachedLasers`
  (params (IDClear :type String))
  (bind (_arrayindex _arrayelement) (`/Engine/EditorBlueprintResources/StandardMacros.ReverseForEachLoop` (`self.LaserAtached`))
    (:`LoopBody`
      (`/Engine/EditorBlueprintResources/StandardMacros.IsValid` _arrayelement
        (:`Is Valid`
          (if (`KismetStringLibrary.Contains` (`/Game/Blueprints/Laser/BP_laser.LaserId` _arrayelement) (`local.IDClear`))
            (`self.K2_DestroyActor` _arrayelement)
            (`KismetArrayLibrary.Array_RemoveItem` (`self.LaserAtached`) _arrayelement)))))))

(fn `LaserBounce`
  (params (LaserHit :type "/Game/Blueprints/Laser/BP_laser Object Reference") (HitResponse :type Boolean) (HitInformation :type "HitResult Structure"))
  (returns (NewLaser :type "/Game/Blueprints/Laser/BP_laser Object Reference"))
  (bind (_bblockinghit _binitialoverlap _time _distance _location _impactpoint _normal _impactnormal _physmat _hitactor _hitcomponent _hitbonename _bonename _hititem _elementindex _faceindex _tracestart) (`GameplayStatics.BreakHitResult` HitInformation))
  (bind _laserhit (`local.LaserHit`))
  (if HitResponse
    (bind _returnvalue (`|SpawnActorFromClass` "/Game/Blueprints/Laser/BP_laser.BP_laser_C" (`KismetMathLibrary.MakeTransform` _impactpoint (`self.CalculateRotation` _impactpoint _normal _tracestart)) "Undefined" "MultiplyWithRoot" null (`/Game/Blueprints/Laser/BP_laser.UpdateID` _laserhit "B") (`/Game/Blueprints/Laser/BP_LaserParent.Color` _laserhit) (`/Game/Blueprints/Laser/BP_LaserParent.SpawnReferance` _laserhit) null))
    (`KismetArrayLibrary.Array_Add` (`self.LaserAtached`) _returnvalue)
    (`KismetArrayLibrary.Array_Add` (`/Game/Blueprints/Laser/BP_LaserSource.ChildLasers` (`/Game/Blueprints/Laser/BP_LaserParent.SpawnReferance` (`local.LaserHit`))) _returnvalue)
    (return _returnvalue)
    (else
      (`self.ClearAtachedLasers` (`/Game/Blueprints/Laser/BP_laser.LaserId` (`local.LaserHit`))))))

(fn `UserConstructionScript`
  (`parent.UserConstructionScript`))