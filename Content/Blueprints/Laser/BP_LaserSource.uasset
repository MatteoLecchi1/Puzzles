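; BP_LaserSource is the emitter actor that starts a chain of BP_laser beams.
; On BeginPlay it spawns the first laser at its Arrow's location with its color, display name as ID and a self reference, then tracks it in ChildLasers.
; RemoveFollowingLasers walks that list backwards, calls CancelTargetHit on lasers whose ID contains the given laser's ID, flagging exact matches, and drops those returning true.
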(event `self.ReceiveBeginPlay`
  (set `self.SpawnReferance` self)
  (set `self.ID` (`KismetSystemLibrary.GetDisplayName` self))
  (bind _returnvalue (`|SpawnActorFromClass` "/Game/Blueprints/Laser/BP_laser.BP_laser_C" (`KismetMathLibrary.MakeTransform` (`SceneComponent.K2_GetComponentLocation` (`self.Arrow`)) (`self.K2_GetActorRotation`)) "Undefined" "MultiplyWithRoot" null (`self.ID`) (`self.Color`) (`self.SpawnReferance`) null))
  (`KismetArrayLibrary.Array_Add` (`self.ChildLasers`) _returnvalue))

(fn `RemoveFollowingLasers`
  (params (laserReferance :type "/Game/Blueprints/Laser/BP_laser Object Reference"))
  (locals (IDRemoved :type String))
  (set `local.IDRemoved` (`/Game/Blueprints/Laser/BP_laser.LaserId` laserReferance))
  (bind (_arrayindex _arrayelement) (`/Engine/EditorBlueprintResources/StandardMacros.ReverseForEachLoop` (`self.ChildLasers`))
    (:`LoopBody`
      (`/Engine/EditorBlueprintResources/StandardMacros.IsValid` _arrayelement
        (:`Is Valid`
          (if (`KismetStringLibrary.Contains` (`/Game/Blueprints/Laser/BP_laser.LaserId` _arrayelement) (`local.IDRemoved`))
            (bind _removefromarray (`/Game/Blueprints/Laser/BP_laser.CancelTargetHit` _arrayelement (`KismetStringLibrary.EqualEqual_StrStr` (`/Game/Blueprints/Laser/BP_laser.LaserId` _arrayelement) (`local.IDRemoved`))))
            (if _removefromarray
              (`KismetArrayLibrary.Array_RemoveItem` (`self.ChildLasers`) _arrayelement))))))))

(fn `UserConstructionScript`)