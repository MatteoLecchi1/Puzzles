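; Laser beam actor that can bounce off mirrors and notify objects it hits through the BP_lasers interface.
; Each tick it traces along its up vector, stretching the mesh and four rect lights to the hit or maximum range.
; Hit changes request or remove follow-on lasers; an unchanged mirror hit repositions and rotates the bounce laser.
; BeginPlay tints the beam, and CancelTargetHit releases the last target, optionally destroying the laser.
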(event `self.ReceiveBeginPlay`
  (`self.ChangeColor`))

(event `self.ReceiveTick`
  (params (DeltaSeconds :type "Float (single-precision)"))
  (`self.SetEndPoint`))

(fn `CancelTargetHit`
  (params (override :type Boolean))
  (returns (RemoveFromArray :type Boolean))
  (`|ExecutionSequence`
    (:`then_0`
      (bind _lasthitactor (`self.LastHitActor`)
        (:`then`
          (bind _asbp_laser_parent (cast `/Game/Blueprints/Laser/BP_LaserParent` _lasthitactor))
          (if (and (`KismetSystemLibrary.DoesImplementInterface` _asbp_laser_parent "/Game/Blueprints/Laser/BP_lasers.BP_lasers_C") (`KismetArrayLibrary.Array_IsEmpty` (`/Game/Blueprints/Laser/BP_LaserParent.LaserAtached` _asbp_laser_parent)))
            (message `/Game/Blueprints/Laser/BP_lasers.LaserBounce` (`self.LastHitActor`) self false (struct))
            (else
              (set `/Game/Blueprints/Laser/BP_LaserParent.isActive` false _asbp_laser_parent))))
        (:`else`)))
    (:`then_1`
      (if override
        (return false)
        (else
          (`self.K2_DestroyActor`)
          (return true))))))

(fn `ChangeColor`
  (bind _returnvalue (`PrimitiveComponent.CreateDynamicMaterialInstance` (`self.StaticMesh`) 0 "/Game/Blueprints/Laser/M_laser.M_laser" "None"))
  (`MaterialInstanceDynamic.SetVectorParameterValue` _returnvalue "Color" (`self.Color`)))

(fn `SetEndPoint`
  (bind _returnvalue (`self.GetActorUpVector`))
  (bind _bouncelaser (`self.bounceLaser`))
  (bind (_bblockinghit _binitialoverlap _time _distance _location _impactpoint _normal _impactnormal _physmat _hitactor _hitcomponent _hitbonename _bonename _hititem _elementindex _faceindex _tracestart) (`GameplayStatics.BreakHitResult` (`self.LaserHitInfo`)))
  (bind _returnvalue_2 (+ (`self.K2_GetActorLocation`) (* _returnvalue 2.0)))
  (bind _outhit (`KismetSystemLibrary.LineTraceSingle` _returnvalue_2 (+ _returnvalue_2 (* _returnvalue (`self.LaserRange`))) "TraceTypeQuery1"))
  (bind _output_get (set `self.LaserHitInfo` _outhit))
  (bind (_bblockinghit_2 _binitialoverlap_2 _time_2 _distance_2 _location_2 _impactpoint_2 _normal_2 _impactnormal_2 _physmat_2 _hitactor_2) (`GameplayStatics.BreakHitResult` _output_get))
  (set `self.Hit Actor` _hitactor_2)
  (bind _returnvalue_3 (`KismetMathLibrary.SelectFloat` (/ (+ _distance_2 1.0) 100.0) (/ (`self.LaserRange`) 100.0) _bblockinghit_2))
  (`SceneComponent.SetWorldScale3D` (`self.StaticMesh`) (`KismetMathLibrary.MakeVector` 0.1 0.1 _returnvalue_3))
  (bind _returnvalue_4 (* _returnvalue_3 64.0))
  (`RectLightComponent.SetSourceHeight` (`self.RectLight`) _returnvalue_4)
  (`RectLightComponent.SetSourceHeight` (`self.RectLight1`) _returnvalue_4)
  (`RectLightComponent.SetSourceHeight` (`self.RectLight2`) _returnvalue_4)
  (`RectLightComponent.SetSourceHeight` (`self.RectLight3`) _returnvalue_4)
  (`self.Hit Actor`
    (:`then`
      (`|ExecutionSequence`
        (:`then_0`
          (if (== (`self.Hit Actor`) (`self.LastHitActor`))
            (bind _asbp_mirror (cast `/Game/Blueprints/Laser/BP_Mirror` (`self.LastHitActor`)))
            (`/Engine/EditorBlueprintResources/StandardMacros.IsValid` _bouncelaser
              (:`Is Valid`
                (`self.K2_SetActorLocation` _bouncelaser _impactpoint false false)
                (`self.K2_SetActorRotation` (`self.bounceLaser`) (`/Game/Blueprints/Laser/BP_Mirror.CalculateRotation` _asbp_mirror _impactpoint _impactnormal _tracestart) false)))
            (else
              (`|ExecutionSequence`
                (:`then_0`
                  (if (`KismetSystemLibrary.DoesImplementInterface` (`self.LastHitActor`) "/Game/Blueprints/Laser/BP_lasers.BP_lasers_C")
                    (`/Game/Blueprints/Laser/BP_LaserSource.RemoveFollowingLasers` (`self.SpawnReferance`) self)))
                (:`then_1`
                  (if (`KismetSystemLibrary.DoesImplementInterface` (`self.Hit Actor`) "/Game/Blueprints/Laser/BP_lasers.BP_lasers_C")
                    (bind _newlaser (message `/Game/Blueprints/Laser/BP_lasers.LaserBounce` (`self.Hit Actor`) self true (`self.LaserHitInfo`)))
                    (set `self.bounceLaser` _newlaser)))))))
        (:`then_1`
          (set `self.LastHitActor` (`self.Hit Actor`)))))
    (:`else`
      (`|ExecutionSequence`
        (:`then_0`
          (bind _lasthitactor (`self.LastHitActor`)
            (:`then`
              (if (`KismetSystemLibrary.DoesImplementInterface` _lasthitactor "/Game/Blueprints/Laser/BP_lasers.BP_lasers_C")
                (message `/Game/Blueprints/Laser/BP_lasers.LaserBounce` (`self.LastHitActor`) self false (`self.LaserHitInfo`))))
            (:`else`)))
        (:`then_1`
          (set `self.LastHitActor` null)
          (set `self.bounceLaser` null))))))

(fn `UpdateID`
  (params (NewString :type String))
  (returns (ReturnValue :type String))
  (return (`KismetStringLibrary.Concat_StrStr` (`self.LaserId`) NewString)))

(fn `UserConstructionScript`)