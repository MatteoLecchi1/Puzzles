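; Pila is an actor that builds a rectangular outline of repeated static mesh components in its construction script.
; VectorTemmie's X and Y set the extent and BaseLenght sets the spacing, with nothing spawned when both X and Y are zero.
; A nested grid loop keeps only edge cells, attaching each new component to StaticMesh at a flat relative offset.
; The event graph holds only disabled stubs, so it has no runtime logic.
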(fn `UserConstructionScript`
  (bind _vectortemmie (`self.vectorTemmie`))
  (bind _baselenght (`self.BaseLenght`))
  (bind _baselenght_2 (`self.BaseLenght`))
  (bind _returnvalue (`KismetMathLibrary.FFloor` (/ (.y _vectortemmie) _baselenght)))
  (bind _returnvalue_2 (`KismetMathLibrary.FFloor` (/ (.x _vectortemmie) _baselenght)))
  (if (`KismetMathLibrary.NotEqualExactly_VectorVector` (* _vectortemmie (1.0 1.0 0.0)))
    (for _index (range (+ _returnvalue_2 1))
      (for _index_2 (range (+ _returnvalue 1))
        (if (or (== _index _returnvalue_2) (== _index_2 _returnvalue) (== _index 0) (== _index_2 0))
          (bind _returnvalue_3 (`AddComponent|NODE_AddStaticMeshComponent-0` :`bManualAttachment` true))
          (`SceneComponent.K2_AttachToComponent` _returnvalue_3 (`self.StaticMesh`) "None" "KeepRelative" "KeepRelative" "KeepRelative" true)
          (`SceneComponent.K2_SetRelativeLocation` _returnvalue_3 (`KismetMathLibrary.MakeVector` (* _index _baselenght_2) (* _index_2 _baselenght_2)) false false))))))