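; BP_Button is a lettered button that sends its letter to every Door sharing its DoorID when activated with the player inside its overlap area.
; On BeginPlay it labels its text widget and caches buttons and doors with that ID.
; Activation starts or rewinds a timeline driving a progress bar and, on first start, shows a light.
; The latest button to start its timer clears the doors' symbols when it finishes.
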(event `self.ReceiveBeginPlay`
  (bind _asbp_button_text (cast `/Game/Blueprints/BP_ButtonText` (`WidgetComponent.GetWidget` (`self.Widget`))))
  (`/Game/Blueprints/BP_ButtonText.UpdateText` _asbp_button_text (`self.Letter`))
  (bind _outactors (`GameplayStatics.GetAllActorsOfClass` "BP_Button_C"))
  (for _array_element _outactors
    (if (== (`/Game/Blueprints/BP_Button.DoorID` _array_element) (`self.DoorID`))
      (`KismetArrayLibrary.Array_Add` (`self.ButtonsWithSameID`) _array_element)))
  (bind _outactors_2 (`GameplayStatics.GetAllActorsOfClass` "/Game/Blueprints/Door.Door_C"))
  (for _array_element_2 _outactors_2
    (if (== (`/Game/Blueprints/Door.DoorID` _array_element_2) (`self.DoorID`))
      (`KismetArrayLibrary.Array_Add` (`self.DoorsWithSameID`) _array_element_2))))

(event `self.InteractArea.OnComponentBeginOverlap`
  (params (OverlappedComponent :type "PrimitiveComponent Object Reference") (OtherActor :type "Actor Object Reference") (OtherComp :type "PrimitiveComponent Object Reference") (OtherBodyIndex :type Integer) (bFromSweep :type Boolean) (SweepResult :type "HitResult Structure (by ref)"))
  (if (== (`GameplayStatics.GetObjectClass` OtherActor) "/Game/ThirdPerson/Blueprints/BP_ThirdPersonCharacter.BP_ThirdPersonCharacter_C")
    (set `self.IsPlayerInArea` true)))

(event `self.InteractArea.OnComponentEndOverlap`
  (params (OverlappedComponent :type "PrimitiveComponent Object Reference") (OtherActor :type "Actor Object Reference") (OtherComp :type "PrimitiveComponent Object Reference") (OtherBodyIndex :type Integer))
  (if (== (`GameplayStatics.GetObjectClass` OtherActor) "/Game/ThirdPerson/Blueprints/BP_ThirdPersonCharacter.BP_ThirdPersonCharacter_C")
    (set `self.IsPlayerInArea` false)))

(event `Activate`
  (if (`self.IsPlayerInArea`)
    (`/Game/Blueprints/Door.Activate` (`self.DoorsWithSameID`) (`self.Letter`))
    (if (`self.IsRunning`)
      (bind (_direction _newtrack_0) (`Timeline|Activation` :!via `SetNewTime` :!label _label)
        (:`Update`
          (bind _asbp_progress_bar (cast `/Game/Blueprints/BP_ProgressBar` (`WidgetComponent.GetWidget` (`self.Progress Bar`))))
          (`/Game/Blueprints/BP_ProgressBar.UpdateBar` _asbp_progress_bar _newtrack_0))
        (:`Finished`
          (if (`self.shouldResetDoor`)
            (`/Game/Blueprints/Door.ClearSymbols` (`self.DoorsWithSameID`)))
          (set `self.IsRunning` false)))
      (else
        (set `self.IsRunning` true)
        (for _array_element (`self.ButtonsWithSameID`)
          (set `/Game/Blueprints/BP_Button.shouldResetDoor` false _array_element))
        (set `self.shouldResetDoor` true)
        (`SceneComponent.SetVisibility` (`self.Luce`) true false)
        (goto _label :!via `PlayFromStart`)))))

(fn `UserConstructionScript`)