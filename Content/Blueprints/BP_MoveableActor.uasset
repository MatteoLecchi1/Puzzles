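; BP_MoveableActor is a movable actor that tracks player proximity and snaps to a 50-unit grid when released.
; Box overlap events set IsPlayerInArea when a BP_ThirdPersonCharacter enters or leaves.
; LetGo subtracts each axis's modulo 50 from the root's world location, truncating toward zero, and sets location and rotation together with no rotation input supplied.
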(event `self.Box.OnComponentBeginOverlap`
  (params (OverlappedComponent :type "PrimitiveComponent Object Reference") (OtherActor :type "Actor Object Reference") (OtherComp :type "PrimitiveComponent Object Reference") (OtherBodyIndex :type Integer) (bFromSweep :type Boolean) (SweepResult :type "HitResult Structure (by ref)"))
  (if (== (`GameplayStatics.GetObjectClass` OtherActor) "/Game/ThirdPerson/Blueprints/BP_ThirdPersonCharacter.BP_ThirdPersonCharacter_C")
    (set `self.IsPlayerInArea` true)))

(event `self.Box.OnComponentEndOverlap`
  (params (OverlappedComponent :type "PrimitiveComponent Object Reference") (OtherActor :type "Actor Object Reference") (OtherComp :type "PrimitiveComponent Object Reference") (OtherBodyIndex :type Integer))
  (if (== (`GameplayStatics.GetObjectClass` OtherActor) "/Game/ThirdPerson/Blueprints/BP_ThirdPersonCharacter.BP_ThirdPersonCharacter_C")
    (set `self.IsPlayerInArea` false)))

(event `LetGo`
  (bind (_returnvalue_x _returnvalue_y _returnvalue_z) (`KismetMathLibrary.BreakVector` (`SceneComponent.K2_GetComponentLocation` (`self.DefaultSceneRoot`))))
  (`SceneComponent.K2_SetWorldLocationAndRotation` :`self` (`self.DefaultSceneRoot`) :`NewLocation` (`KismetMathLibrary.MakeVector` (- _returnvalue_x (mod _returnvalue_x 50.0)) (- _returnvalue_y (mod _returnvalue_y 50.0)) (- _returnvalue_z (mod _returnvalue_z 50.0)))))

(fn `UserConstructionScript`)