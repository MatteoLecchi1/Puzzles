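; Lever actor that swaps world objects sharing its ObjectID and redirects the central lamp's light target.
; Pull searches SwappableActors interface implementers, calls SwapActorMessage on matches, and aims every BP_CentralLamp at the swapped actor, or back at itself if the actor was already modified.
; A separate Rotate event turns the Cube 180 degrees.
; Box overlaps track the player's presence and toggle the button prompt.
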(event `Pull`
  (bind _outactors (`GameplayStatics.GetAllActorsWithInterface` "/Game/Blueprints/Lenses/SwappableActors.SwappableActors_C"))
  (for _array_element _outactors
    (bind _asbp_swappale_actor_parent (cast `/Game/Blueprints/Lenses/BP_SwappaleActorParent` _array_element))
    (if (== (`/Game/Blueprints/Lenses/BP_SwappaleActorParent.ObjectID` _asbp_swappale_actor_parent) (`self.ObjectID`))
      (if (`/Game/Blueprints/Lenses/BP_SwappaleActorParent.isInModifiedState` _asbp_swappale_actor_parent)
        (message `/Game/Blueprints/Lenses/SwappableActors.Swap Actor` _asbp_swappale_actor_parent)
        (bind _outactors_2 (`GameplayStatics.GetAllActorsOfClass` "/Game/Blueprints/Lenses/BP_CentralLamp.BP_CentralLamp_C"))
        (for _array_element_2 _outactors_2
          (set `/Game/Blueprints/Lenses/BP_CentralLamp.LightTarget` _array_element_2 _array_element_2))
        (else
          (message `/Game/Blueprints/Lenses/SwappableActors.Swap Actor` _asbp_swappale_actor_parent)
          (bind _outactors_3 (`GameplayStatics.GetAllActorsOfClass` "/Game/Blueprints/Lenses/BP_CentralLamp.BP_CentralLamp_C"))
          (for _array_element_3 _outactors_3
            (set `/Game/Blueprints/Lenses/BP_CentralLamp.LightTarget` _asbp_swappale_actor_parent _array_element_3)))))))

(event `Rotate`
  (`SceneComponent.K2_AddRelativeRotation` (`self.Cube`) (struct :`Yaw` 180.0) false false))

(event `self.Box.OnComponentBeginOverlap`
  (params (OverlappedComponent :type "PrimitiveComponent Object Reference") (OtherActor :type "Actor Object Reference") (OtherComp :type "PrimitiveComponent Object Reference") (OtherBodyIndex :type Integer) (bFromSweep :type Boolean) (SweepResult :type "HitResult Structure (by ref)"))
  (if (== OtherActor (`GameplayStatics.GetPlayerCharacter` 0))
    (bind _output_get (set `self.IsPlayerInArea` true))
    (`SceneComponent.SetVisibility` (`self.ButtonPrompt`) _output_get false)))

(event `self.Box.OnComponentEndOverlap`
  (params (OverlappedComponent :type "PrimitiveComponent Object Reference") (OtherActor :type "Actor Object Reference") (OtherComp :type "PrimitiveComponent Object Reference") (OtherBodyIndex :type Integer))
  (if (== OtherActor (`GameplayStatics.GetPlayerCharacter` 0))
    (bind _output_get (set `self.IsPlayerInArea` false))
    (`SceneComponent.SetVisibility` (`self.ButtonPrompt`) _output_get false)))

(fn `UserConstructionScript`)