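; Lens-modifiable cube that becomes a walking cube, pacing back and forth along its forward axis while in its modified state.
; Each Tick, short Visibility line traces from Center check ahead, then behind, setting the Reverse sign to head away from whatever is hit.
; It moves at constant speed through SetActorLocation without sweep, so the traces alone handle obstacle detection.
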(event `self.ReceiveTick`
  (params (DeltaSeconds :type "Float (single-precision)"))
  (bind _returnvalue (`SceneComponent.K2_GetComponentLocation` (`self.Center`)))
  (bind _returnvalue_2 (* (`self.GetActorForwardVector`) 100.0))
  (`parent.ReceiveTick` DeltaSeconds)
  (if (`self.isInModifiedState`)
    (bind (_outhit _returnvalue_3) (`KismetSystemLibrary.LineTraceSingle` _returnvalue (+ _returnvalue _returnvalue_2) "TraceTypeQuery1"))
    (if _returnvalue_3
      (set `self.Reverse` -1.0)
      (else
        (bind (_outhit_2 _returnvalue_4) (`KismetSystemLibrary.LineTraceSingle` _returnvalue (+ _returnvalue (* _returnvalue_2 -1.0)) "TraceTypeQuery1"))
        (if _returnvalue_4
          (set `self.Reverse` 1.0))))
    (`self.K2_SetActorLocation` self (+ (* (`self.GetActorForwardVector`) 150.0 DeltaSeconds (`self.Reverse`)) (`self.K2_GetActorLocation`)) false false)))

(fn `UserConstructionScript`
  (`parent.UserConstructionScript`))