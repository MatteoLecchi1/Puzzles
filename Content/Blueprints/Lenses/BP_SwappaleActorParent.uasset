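; Parent actor for swappable objects that toggle between a normal and a modified static mesh, each state with its own movable flag.
; SwapActor reverts other modified actors before modifying this one, so normally only one is modified at once.
; SwapStaticMesh, blocked while held or unsafe, flips visibility and collision, then rotates BP_LampLevers with matching ObjectID and refreshes grab/rotate prompts.
; BeginPlay swaps twice to initialize state; preview hooks are empty.
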(event `self.ReceiveBeginPlay`
  (set `self.MeshNormal` (`self.StaticMeshNormal`))
  (set `self.MeshModified` (`self.StaticMeshModified`))
  (`self.SwapStaticMesh`)
  (`self.SwapStaticMesh`))

(event `/Game/Blueprints/Lenses/SwappableActors.Swap Actor`
  (if (`self.isInModifiedState`)
    (`self.SwapStaticMesh`)
    (else
      (bind _outactors (`GameplayStatics.GetAllActorsWithInterface` "/Game/Blueprints/Lenses/SwappableActors.SwappableActors_C"))
      (for _array_element _outactors
        (bind _asbp_swappale_actor_parent (cast `/Game/Blueprints/Lenses/BP_SwappaleActorParent` _array_element))
        (if (`/Game/Blueprints/Lenses/BP_SwappaleActorParent.isInModifiedState` _asbp_swappale_actor_parent)
          (`self.SwapStaticMesh` _asbp_swappale_actor_parent)))
      (`self.SwapStaticMesh`))))

(event `/Game/Blueprints/Lenses/SwappableActors.ChangeToPreview`)

(event `self.UpdateUIVisibility`
  (bind _buttongrabprompt (`self.ButtonGrabPrompt`))
  (if (`self.IsPlayerInArea`)
    (if (`self.isInModifiedState`)
      (if (`self.IsModifiedMovable`)
        (`SceneComponent.SetVisibility` _buttongrabprompt true false :!label _label)
        (else
          (`SceneComponent.SetVisibility` _buttongrabprompt false false :!label _label_2)))
      (elif (`self.IsNormalMovable`)
        (goto _label)
        (else
          (goto _label_2))))
    (else
      (goto _label_2)))
  (`SceneComponent.SetVisibility` (`self.ButtonRotatePrompt`) (`self.isBeingHeld`) false))

(fn `Preview`)

(fn `SwapStaticMesh`
  (locals (NewLocalVar :type Boolean))
  (bind _meshnormal (`self.MeshNormal`))
  (bind _meshnormal_2 (`self.MeshNormal`))
  (bind _meshmodified (`self.MeshModified`))
  (bind _meshmodified_2 (`self.MeshModified`))
  (if (`self.isSafeToSwap`)
    (if (not (`self.isBeingHeld`))
      (if (`self.isInModifiedState`)
        (`SceneComponent.SetVisibility` _meshmodified_2 false true)
        (`PrimitiveComponent.SetCollisionEnabled` _meshmodified_2 "NoCollision")
        (`SceneComponent.SetVisibility` _meshnormal_2 true true)
        (`PrimitiveComponent.SetCollisionEnabled` _meshnormal_2 "QueryAndPhysics")
        (set `self.isInModifiedState` false)
        (set `self.IsMovable` (`self.IsNormalMovable`))
        (else
          (`SceneComponent.SetVisibility` _meshmodified true true)
          (`PrimitiveComponent.SetCollisionEnabled` _meshmodified "QueryAndPhysics")
          (`SceneComponent.SetVisibility` _meshnormal false true)
          (`PrimitiveComponent.SetCollisionEnabled` _meshnormal "NoCollision")
          (set `self.isInModifiedState` true)
          (set `self.IsMovable` (`self.IsModifiedMovable`))))
      (bind _outactors (`GameplayStatics.GetAllActorsOfClass` "/Game/Blueprints/Lenses/BP_LampLever.BP_LampLever_C"))
      (for _array_element _outactors
        (if (== (`/Game/Blueprints/Lenses/BP_LampLever.ObjectID` _array_element) (`self.ObjectID`))
          (`/Game/Blueprints/Lenses/BP_LampLever.Rotate` _array_element)
          (`self.UpdateUIVisibility`))))))

(fn `UserConstructionScript`)