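; A door that opens once the required sequence of symbols has been entered, by destroying its Cube component.
; On BeginPlay it shows the joined required symbols through a BP_ButtonText widget.
; Activate appends a received symbol to the current entry if it appears anywhere in the required set, then compares both joined strings, so order matters.
; ClearSymbols empties the current entry.
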(event `self.ReceiveBeginPlay`
  (bind _asbp_button_text (cast `/Game/Blueprints/BP_ButtonText` (`WidgetComponent.GetWidget` (`self.Text`))))
  (`/Game/Blueprints/BP_ButtonText.UpdateText` _asbp_button_text (`KismetStringLibrary.JoinStringArray` (`self.Symbols`) "")))

(event `Activate`
  (params (Symbol :type String))
  (bind _symbols (`self.Symbols`))
  (bind _currentsymbols (`self.CurrentSymbols`))
  (bind _returnvalue (`KismetStringLibrary.JoinStringArray` _currentsymbols ""))
  (set `self.SymbolFound` false)
  (for _array_element _symbols
    (if (and (`KismetStringLibrary.EqualEqual_StrStr` Symbol _array_element) (not (`self.SymbolFound`)))
      (`KismetArrayLibrary.Array_Add` _currentsymbols _array_element)
      (set `self.SymbolFound` true)
      (`KismetSystemLibrary.PrintString` _returnvalue)
      (if (`KismetStringLibrary.EqualEqual_StrStr` (`KismetStringLibrary.JoinStringArray` _symbols "") _returnvalue)
        (`ActorComponent.K2_DestroyComponent` (`self.Cube`))))))

(event `ClearSymbols`
  (`KismetArrayLibrary.Array_Clear` (`self.CurrentSymbols`)))

(fn `UserConstructionScript`)